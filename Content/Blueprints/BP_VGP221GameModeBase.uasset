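; Game mode that populates the level on BeginPlay and drives the start, pause, game-end and restart flow.
; It shuffles spawner actors to place up to ten turrets, alternating two types or random when spawners are scarce, and a small fixed mix of collectibles.
; It creates all UI widgets up front, opens paused on the start menu, and toggles widgets, pause and mouse cursor for each state.
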(event `self.ReceiveBeginPlay`
  (`self.SpawnTurrets`)
  (`self.SpawnPickups`)
  (add `self.CallGameEnd` (delegate `GameEnd`))
  (`self.CreateWidgets`))

(event `GameEnd`
  (`UserWidget.AddToViewport` (`self.GameEndWidget`) 0)
  (`GameplayStatics.SetGamePaused` true)
  (set `PlayerController.bShowMouseCursor` true (`GameplayStatics.GetPlayerController` 0)))

(fn `CreateWidgets`
  (bind _returnvalue (`|CreateWidget` "/Game/Blueprints/UI/BP_PrimaryUIWidget.BP_PrimaryUIWidget_C"))
  (set `self.UIWidget` _returnvalue)
  (bind _returnvalue_2 (`|CreateWidget` "/Game/Blueprints/UI/GameEndWidget.GameEndWidget_C"))
  (set `self.GameEndWidget` _returnvalue_2)
  (bind _returnvalue_3 (`|CreateWidget` "/Game/Blueprints/UI/PauseMenuWidget.PauseMenuWidget_C"))
  (set `self.PauseWidget` _returnvalue_3)
  (bind _returnvalue_4 (`|CreateWidget` "/Game/Blueprints/UI/StartMenuWidget.StartMenuWidget_C"))
  (bind _output_get (set `self.StartWidget` _returnvalue_4))
  (`UserWidget.AddToViewport` _output_get 0)
  (`GameplayStatics.SetGamePaused` true)
  (set `PlayerController.bShowMouseCursor` true (`GameplayStatics.GetPlayerController` 0)))

(fn `Pause Game`
  (`UserWidget.AddToViewport` (`self.PauseWidget`) 0)
  (`GameplayStatics.SetGamePaused` true)
  (set `PlayerController.bShowMouseCursor` true (`GameplayStatics.GetPlayerController` 0)))

(fn `RestartLevel`
  (bind _returnvalue (`GameplayStatics.GetCurrentLevelName` true))
  (`GameplayStatics.OpenLevel` (`KismetStringLibrary.Conv_StringToName` _returnvalue)))

(fn `Resume Game`
  (`Widget.RemoveFromParent` (`self.PauseWidget`))
  (`GameplayStatics.SetGamePaused` false)
  (set `PlayerController.bShowMouseCursor` false (`GameplayStatics.GetPlayerController` 0)))

(fn `SpawnPickups`
  (bind _outactors (`GameplayStatics.GetAllActorsOfClass` "/Game/Blueprints/Pickups/BP_CollectibleSpawner.BP_CollectibleSpawner_C"))
  (`KismetArrayLibrary.Array_Shuffle` _outactors)
  (for (_array_element _array_index) _outactors
    (if (< _array_index 2)
      (`CollectibleSpawner.SpawnCollectible` _array_element false 0)
      (elif (< _array_index 3)
        (`CollectibleSpawner.SpawnCollectible` _array_element false 1)
        (else
          (break))))))

(fn `SpawnTurrets`
  (bind _outactors (`GameplayStatics.GetAllActorsOfClass` "/Game/Blueprints/Enemies/BP_TurretSpawner.BP_TurretSpawner_C"))
  (if (> (`KismetArrayLibrary.Array_Length` _outactors) 10)
    (`KismetArrayLibrary.Array_Shuffle` _outactors)
    (for (_array_element _array_index) _outactors
      (if (< _array_index 10)
        (`TurretSpawner.SpawnTurret` _array_element false (mod _array_index 2))
        (else
          (break))))
    (else
      (for _array_element_2 _outactors
        (`TurretSpawner.SpawnTurret` _array_element_2 true 0)))))

(fn `StartGame`
  (`Widget.RemoveFromParent` (`self.StartWidget`))
  (`UserWidget.AddToViewport` (`self.UIWidget`) 0)
  (`GameplayStatics.SetGamePaused` false)
  (set `PlayerController.bShowMouseCursor` false (`GameplayStatics.GetPlayerController` 0)))

(fn `UserConstructionScript`)