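; Cannon turret enemy Blueprint whose graph drives a floating health bar.
; On BeginPlay it caches the HP widget and binds to UpdateHealthBar to push the Health to MaxHealth ratio.
; Each Tick it traces on the Camera channel from the bar toward the player, ignoring projectiles gathered by a per-frame actor search.
; The bar shows and faces the camera only when the trace hits the FPSCharacter, otherwise it hides.
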(event `self.ReceiveBeginPlay`
  (bind _asbp_hpwidget (cast `/Game/Blueprints/UI/BP_HPWidget` (`WidgetComponent.GetWidget` (`self.HealthBarWidget`))))
  (set `self.HPWidget` _asbp_hpwidget)
  (add `self.UpdateHealthBar` (delegate `UpdateHealthBar_Event_0`)))

(event `UpdateHealthBar_Event_0`
  (`/Game/Blueprints/UI/BP_HPWidget.UpdateHealth` (`self.HPWidget`) (/ (`self.Health`) (`self.MaxHealth`))))

(event `self.ReceiveTick`
  (params (DeltaSeconds :type "Float (single-precision)"))
  (bind _healthbarwidget (`self.HealthBarWidget`))
  (bind _returnvalue (`SceneComponent.K2_GetComponentLocation` (`self.HealthBarWidget`)))
  (bind _outactors (`GameplayStatics.GetAllActorsOfClass` "/Script/VGP221.Projectile"))
  (bind _outhit (`KismetSystemLibrary.LineTraceSingle` _returnvalue (+ (* (`KismetMathLibrary.Normal` (- (`self.K2_GetActorLocation` (`GameplayStatics.GetPlayerCharacter` 0)) _returnvalue)) (`self.MaxDistance`)) _returnvalue) "TraceTypeQuery2" false _outactors))
  (cast `FPSCharacter` (`.HitActor` (`GameplayStatics.BreakHitResult` _outhit))
    (:`then`
      (`SceneComponent.SetVisibility` _healthbarwidget true false)
      (`SceneComponent.K2_SetRelativeRotation` _healthbarwidget (`KismetMathLibrary.FindLookAtRotation` (`SceneComponent.K2_GetComponentLocation` _healthbarwidget) (`PlayerCameraManager.GetCameraLocation` (`GameplayStatics.GetPlayerCameraManager` 0))) false false))
    (:`CastFailed`
      (`SceneComponent.SetVisibility` _healthbarwidget false false))))

(fn `UserConstructionScript`)